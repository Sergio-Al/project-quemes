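; BP_PushableBase is a cube actor that the TopDownCharacter can push.
; Separate X-axis and Y-axis collision components detect the character and call its SettingPushing on begin overlap and StopPushing on end overlap.
; Both begin and end overlaps enable physics simulation on the cube, and nothing in these graphs turns it off.
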(event `self.YAxisCollision.OnComponentBeginOverlap`
  (params (OverlappedComponent :type "PrimitiveComponent Object Reference") (OtherActor :type "Actor Object Reference") (OtherComp :type "PrimitiveComponent Object Reference") (OtherBodyIndex :type Integer) (bFromSweep :type Boolean) (SweepResult :type "HitResult Structure (by ref)"))
  ;[1 1 1] Y Axis Collision
  (bind _astop_down_character (cast `/Game/Characters/TopDownBP/Blueprints/TopDownCharacter` OtherActor))
  (`PrimitiveComponent.SetSimulatePhysics` (`self.MyCube`) true)
  (`/Game/Characters/TopDownBP/Blueprints/TopDownCharacter.SettingPushing` _astop_down_character))

(event `self.YAxisCollision.OnComponentEndOverlap`
  (params (OverlappedComponent :type "PrimitiveComponent Object Reference") (OtherActor :type "Actor Object Reference") (OtherComp :type "PrimitiveComponent Object Reference") (OtherBodyIndex :type Integer))
  ;[1 1 1] Y Axis Collision
  (bind _astop_down_character (cast `/Game/Characters/TopDownBP/Blueprints/TopDownCharacter` OtherActor))
  (`PrimitiveComponent.SetSimulatePhysics` (`self.MyCube`) true)
  (`/Game/Characters/TopDownBP/Blueprints/TopDownCharacter.StopPushing` _astop_down_character))

(event `self.XAxisCollision.OnComponentBeginOverlap`
  (params (OverlappedComponent :type "PrimitiveComponent Object Reference") (OtherActor :type "Actor Object Reference") (OtherComp :type "PrimitiveComponent Object Reference") (OtherBodyIndex :type Integer) (bFromSweep :type Boolean) (SweepResult :type "HitResult Structure (by ref)"))
  ;[1 1 1] X Axis Component pushing
  (bind _astop_down_character (cast `/Game/Characters/TopDownBP/Blueprints/TopDownCharacter` OtherActor))
  (`PrimitiveComponent.SetSimulatePhysics` (`self.MyCube`) true)
  (`/Game/Characters/TopDownBP/Blueprints/TopDownCharacter.SettingPushing` _astop_down_character))

(event `self.XAxisCollision.OnComponentEndOverlap`
  (params (OverlappedComponent :type "PrimitiveComponent Object Reference") (OtherActor :type "Actor Object Reference") (OtherComp :type "PrimitiveComponent Object Reference") (OtherBodyIndex :type Integer))
  ;[1 1 1] X Axis Component pushing
  (bind _astop_down_character (cast `/Game/Characters/TopDownBP/Blueprints/TopDownCharacter` OtherActor))
  (`PrimitiveComponent.SetSimulatePhysics` (`self.MyCube`) true)
  (`/Game/Characters/TopDownBP/Blueprints/TopDownCharacter.StopPushing` _astop_down_character))

(fn `UserConstructionScript`)